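; BP_ArrayAlongSpline is a construction-script tool that repeats a mesh along a spline.
; It adds one collision-free, X-forward spline mesh component for each XLength step that fits in the spline's length.
; Each segment spans consecutive distances, with tangent length clamped to XLength, but both tangents are always sampled at distance zero.
; XLength is a variable, as the mesh-bounds width calculation is left unused.
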(fn `UserConstructionScript`
  (bind _x_length (`self.X length`))
  (bind _spline (`self.Spline`))
  (bind _spline_2 (`self.Spline`))
  (bind _x_length_2 (`self.X length`))
  (bind _output_get (set `self.X length` (`self.X length`)))
  (for _index (range (+ (`KismetMathLibrary.FTrunc` (/ (`SplineComponent.GetSplineLength` (`self.Spline`)) _output_get)) 1))
    (bind _returnvalue (`AddComponent|NODE_AddSplineMeshComponent-0`))
    (`PrimitiveComponent.SetCollisionEnabled` _returnvalue "NoCollision")
    (`SplineMeshComponent.SetForwardAxis` _returnvalue "X" true)
    (`StaticMeshComponent.SetStaticMesh` _returnvalue (`self.Mesh`))
    (`SplineMeshComponent.SetStartAndEnd` _returnvalue (`SplineComponent.GetLocationAtDistanceAlongSpline` _spline_2 (* _index (`self.X length`)) "Local") (`KismetMathLibrary.ClampVectorSize` (`SplineComponent.GetTangentAtDistanceAlongSpline` _spline_2 0.0 "Local") _x_length _x_length) (`SplineComponent.GetLocationAtDistanceAlongSpline` _spline (* (+ _index 1) (`self.X length`)) "Local") (`KismetMathLibrary.ClampVectorSize` (`SplineComponent.GetTangentAtDistanceAlongSpline` _spline 0.0 "Local") _x_length_2 _x_length_2) true)))